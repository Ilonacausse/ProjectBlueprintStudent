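; Player character Blueprint that drives a head-bob camera effect based on movement.
; Each tick, the head oscillator starts a camera shake on the first player controller.
; It branches three ways: moving below a speed threshold, moving at or above it, or otherwise when stationary or unable to jump.
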(event `Head_Oscillator`
  (bind _returnvalue (`GameplayStatics.GetPlayerController` 0))
  (bind _returnvalue_2 (`KismetMathLibrary.VSize` (`self.GetVelocity`)))
  ;[1 1 1] Camera Oscillator
  (if (and (> _returnvalue_2 0.0) (`self.CanJump`))
    (if (< _returnvalue_2 200.0)
      (`PlayerController.ClientStartCameraShake` :`self` _returnvalue)
      (else
        (`PlayerController.ClientStartCameraShake` :`self` _returnvalue)))
    (else
      (`PlayerController.ClientStartCameraShake` :`self` _returnvalue))))

(event `self.ReceiveTick`
  (params (DeltaSeconds :type "Float (single-precision)"))
  ;[1 1 1] Camera Oscillator
  (`self.Head_Oscillator`))

(fn `UserConstructionScript`)